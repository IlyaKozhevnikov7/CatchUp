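; Player character Blueprint for CatchUp, with key-driven toggles for its appearance and camera.
; Q flip-flops the mesh and Anim Blueprint between Catcher and Runner, while C flip-flops between the default camera and a third-person camera.
; On landing it stores vertical velocity in LastLandedZ and clears it after a very short delay, a stopgap workaround for animation.
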(event EventOnLanded
  (params (Hit :type Hit%20Result%20Structure%20%28by%20ref%29))
  ;[1 1 1] Пока вот такой костыль для анимации
  (Variables|Default|SetLastLandedZ (.z (Transformation|GetVelocity)))
  (Utilities|FlowControl|Delay 0.01)
  (Variables|Default|SetLastLandedZ 0.0))

(event Input|KeyboardEvents|Q
  (params (Key :type Key%20Structure :default "None"))
  (bind _mesh (Variables|Character|GetMesh))
  (bind _mesh_2 (Variables|Character|GetMesh))
  (:Pressed
    (Utilities|FlowControl|FlipFlop
      (:A
        (Class|SkinnedMeshComponent|SetSkeletalMesh _mesh_2 "/Game/CatchUp/Meshes/Game/Player/Catcher/SM_Catcher.SM_Catcher" false)
        (Class|SkeletalMeshComponent|SetAnimClass _mesh_2 "/Game/CatchUp/Animations/Game/Player/Catcher/ABP_Catcher.ABP_Catcher_C"))
      (:B
        (Class|SkinnedMeshComponent|SetSkeletalMesh _mesh "/Game/CatchUp/Meshes/Game/Player/Runer/SM_Runner.SM_Runner" false)
        (Class|SkeletalMeshComponent|SetAnimClass _mesh "/Game/CatchUp/Animations/Game/Player/Runner/ABP_Runner.ABP_Runner_C")))))

(event Input|KeyboardEvents|C
  (params (Key :type Key%20Structure :default "None"))
  (:Pressed
    (Utilities|FlowControl|FlipFlop
      (:A
        (Components|Activation|SetActive (Variables|Default|GetCamera) false true)
        (Components|Activation|SetActive (Variables|Default|Get3pCamera) true true))
      (:B
        (Components|Activation|SetActive (Variables|Default|Get3pCamera) false true)
        (Components|Activation|SetActive (Variables|Default|GetCamera) true true)))))

(fn ConstructionScript)